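; BP_Rain is a rain controller that keeps a Niagara effect and the MPC_Rain material parameter collection in sync through one RainAmount value.
; It writes RainAmount to the collection, reads it back and passes it to the Niagara component's parameter of the same name.
; The construction script applies this when it runs, and a looping timer started at BeginPlay repeats it several times a second instead of using Tick.
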(event `self.ReceiveBeginPlay`
  (`KismetSystemLibrary.K2_SetTimer` null "E_Rain" 0.2 true))

(event `E_Rain`
  (`KismetMaterialLibrary.SetScalarParameterValue` "/Game/WWITrench/Materials/Functions/MPC_Rain.MPC_Rain" "RainAmount" (`self.RainAmount`))
  (bind _returnvalue (`KismetMaterialLibrary.GetScalarParameterValue` "/Game/WWITrench/Materials/Functions/MPC_Rain.MPC_Rain" "RainAmount"))
  (`FXSystemComponent.SetFloatParameter` (`self.Niagara`) "RainAmount" _returnvalue))

(fn `UserConstructionScript`
  (`KismetMaterialLibrary.SetScalarParameterValue` "/Game/WWITrench/Materials/Functions/MPC_Rain.MPC_Rain" "RainAmount" (`self.RainAmount`))
  (bind _returnvalue (`KismetMaterialLibrary.GetScalarParameterValue` "/Game/WWITrench/Materials/Functions/MPC_Rain.MPC_Rain" "RainAmount"))
  (`FXSystemComponent.SetFloatParameter` (`self.Niagara`) "RainAmount" _returnvalue))